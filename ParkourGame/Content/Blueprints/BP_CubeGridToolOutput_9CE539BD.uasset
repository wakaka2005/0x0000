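; Runnable wall actor that tells overlapping actors where a wall run starts and ends.
; Four trigger boxes form two pairs, Box1/Box2 and Box3/Box4, each box targeting its partner so runs work in either direction.
; On begin overlap, SetRunnableWallMessage sends the box transform and partner location with Enable false.
; End overlap sends a zero target with Enable true.
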(event `self.Box1.OnComponentBeginOverlap`
  (params (OverlappedComponent :type "PrimitiveComponent Object Reference") (OtherActor :type "Actor Object Reference") (OtherComp :type "PrimitiveComponent Object Reference") (OtherBodyIndex :type Integer) (bFromSweep :type Boolean) (SweepResult :type "HitResult Structure (by ref)"))
  (message `/Game/_01/BP/Player/BPI_WallRunner.SetRunnableWall` OtherActor (`SceneComponent.K2_GetComponentLocation` (`self.Box2`)) (`SceneComponent.K2_GetComponentToWorld` (`self.Box1`)) false))

(event `self.Box1.OnComponentEndOverlap`
  (params (OverlappedComponent :type "PrimitiveComponent Object Reference") (OtherActor :type "Actor Object Reference") (OtherComp :type "PrimitiveComponent Object Reference") (OtherBodyIndex :type Integer))
  (message `/Game/_01/BP/Player/BPI_WallRunner.SetRunnableWall` OtherActor (0.0 0.0 0.0) (struct) true))

(event `self.Box2.OnComponentBeginOverlap`
  (params (OverlappedComponent :type "PrimitiveComponent Object Reference") (OtherActor :type "Actor Object Reference") (OtherComp :type "PrimitiveComponent Object Reference") (OtherBodyIndex :type Integer) (bFromSweep :type Boolean) (SweepResult :type "HitResult Structure (by ref)"))
  (message `/Game/_01/BP/Player/BPI_WallRunner.SetRunnableWall` OtherActor (`SceneComponent.K2_GetComponentLocation` (`self.Box1`)) (`SceneComponent.K2_GetComponentToWorld` (`self.Box2`)) false))

(event `self.Box2.OnComponentEndOverlap`
  (params (OverlappedComponent :type "PrimitiveComponent Object Reference") (OtherActor :type "Actor Object Reference") (OtherComp :type "PrimitiveComponent Object Reference") (OtherBodyIndex :type Integer))
  (message `/Game/_01/BP/Player/BPI_WallRunner.SetRunnableWall` OtherActor (0.0 0.0 0.0) (struct) true))

(event `self.Box3.OnComponentEndOverlap`
  (params (OverlappedComponent :type "PrimitiveComponent Object Reference") (OtherActor :type "Actor Object Reference") (OtherComp :type "PrimitiveComponent Object Reference") (OtherBodyIndex :type Integer))
  (message `/Game/_01/BP/Player/BPI_WallRunner.SetRunnableWall` OtherActor (0.0 0.0 0.0) (struct) true))

(event `self.Box3.OnComponentBeginOverlap`
  (params (OverlappedComponent :type "PrimitiveComponent Object Reference") (OtherActor :type "Actor Object Reference") (OtherComp :type "PrimitiveComponent Object Reference") (OtherBodyIndex :type Integer) (bFromSweep :type Boolean) (SweepResult :type "HitResult Structure (by ref)"))
  (message `/Game/_01/BP/Player/BPI_WallRunner.SetRunnableWall` OtherActor (`SceneComponent.K2_GetComponentLocation` (`self.Box4`)) (`SceneComponent.K2_GetComponentToWorld` (`self.Box3`)) false))

(event `self.Box4.OnComponentBeginOverlap`
  (params (OverlappedComponent :type "PrimitiveComponent Object Reference") (OtherActor :type "Actor Object Reference") (OtherComp :type "PrimitiveComponent Object Reference") (OtherBodyIndex :type Integer) (bFromSweep :type Boolean) (SweepResult :type "HitResult Structure (by ref)"))
  (message `/Game/_01/BP/Player/BPI_WallRunner.SetRunnableWall` OtherActor (`SceneComponent.K2_GetComponentLocation` (`self.Box3`)) (`SceneComponent.K2_GetComponentToWorld` (`self.Box4`)) false))

(event `self.Box4.OnComponentEndOverlap`
  (params (OverlappedComponent :type "PrimitiveComponent Object Reference") (OtherActor :type "Actor Object Reference") (OtherComp :type "PrimitiveComponent Object Reference") (OtherBodyIndex :type Integer))
  (message `/Game/_01/BP/Player/BPI_WallRunner.SetRunnableWall` OtherActor (0.0 0.0 0.0) (struct) true))

(fn `UserConstructionScript`)