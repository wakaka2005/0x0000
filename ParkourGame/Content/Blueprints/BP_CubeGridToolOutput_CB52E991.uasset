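; A trap floor that drops when the player character steps on it, kills the character, then resets.
; Many trigger boxes run duplicated overlap chains behind a shared HasFallen guard, enabling mesh physics, detaching the character and calling Die after short delays.
; ResetFloor stops physics and restores the actor transform saved at BeginPlay; Box1 alone waits far longer before resetting.
; StepLocation records the character's position but is never read here.
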(event `self.ReceiveBeginPlay`
  (bind _returnvalue (`self.K2_GetActorLocation`))
  (set `self.InitialLocation` _returnvalue)
  (bind _returnvalue_2 (`self.K2_GetActorRotation`))
  (set `self.InitialRotation` _returnvalue_2))

(event `self.Box.OnComponentBeginOverlap`
  (params (OverlappedComponent :type "PrimitiveComponent Object Reference") (OtherActor :type "Actor Object Reference") (OtherComp :type "PrimitiveComponent Object Reference") (OtherBodyIndex :type Integer) (bFromSweep :type Boolean) (SweepResult :type "HitResult Structure (by ref)"))
  (if (not (`self.HasFallen`))
    (bind _asbp_third_person_character (cast `/Game/_01/BP/Player/BP_ThirdPersonCharacter` OtherActor))
    (set `self.AttachedCharacter` null)
    (set `self.HasFallen` true)
    (bind _returnvalue (`self.K2_GetActorLocation` _asbp_third_person_character))
    (set `self.StepLocation` _returnvalue)
    (`KismetSystemLibrary.Delay` 0.2)
    (`PrimitiveComponent.SetSimulatePhysics` (`self.StaticMesh`) true)
    (`PrimitiveComponent.SetEnableGravity` (`self.StaticMesh`) true)
    (`KismetSystemLibrary.Delay` 0.2)
    (`self.K2_DetachFromActor` _asbp_third_person_character "KeepRelative" "KeepRelative" "KeepRelative")
    (`KismetSystemLibrary.Delay` 0.2)
    (`/Game/_01/BP/Player/BP_ThirdPersonCharacter.Die` _asbp_third_person_character)
    (`KismetSystemLibrary.Delay` 0.2)
    (`self.ResetFloor`)))

(event `self.Box2.OnComponentBeginOverlap`
  (params (OverlappedComponent :type "PrimitiveComponent Object Reference") (OtherActor :type "Actor Object Reference") (OtherComp :type "PrimitiveComponent Object Reference") (OtherBodyIndex :type Integer) (bFromSweep :type Boolean) (SweepResult :type "HitResult Structure (by ref)"))
  (if (not (`self.HasFallen`))
    (bind _asbp_third_person_character (cast `/Game/_01/BP/Player/BP_ThirdPersonCharacter` OtherActor))
    (set `self.AttachedCharacter` null)
    (set `self.HasFallen` true)
    (bind _returnvalue (`self.K2_GetActorLocation` _asbp_third_person_character))
    (set `self.StepLocation` _returnvalue)
    (`KismetSystemLibrary.Delay` 0.2)
    (`PrimitiveComponent.SetSimulatePhysics` (`self.StaticMesh`) true)
    (`PrimitiveComponent.SetEnableGravity` (`self.StaticMesh`) true)
    (`KismetSystemLibrary.Delay` 0.2)
    (`self.K2_DetachFromActor` _asbp_third_person_character "KeepRelative" "KeepRelative" "KeepRelative")
    (`KismetSystemLibrary.Delay` 0.2)
    (`/Game/_01/BP/Player/BP_ThirdPersonCharacter.Die` _asbp_third_person_character)
    (`KismetSystemLibrary.Delay` 0.2)
    (`self.ResetFloor`)))

(event `self.Box3.OnComponentBeginOverlap`
  (params (OverlappedComponent :type "PrimitiveComponent Object Reference") (OtherActor :type "Actor Object Reference") (OtherComp :type "PrimitiveComponent Object Reference") (OtherBodyIndex :type Integer) (bFromSweep :type Boolean) (SweepResult :type "HitResult Structure (by ref)"))
  (if (not (`self.HasFallen`))
    (bind _asbp_third_person_character (cast `/Game/_01/BP/Player/BP_ThirdPersonCharacter` OtherActor))
    (set `self.AttachedCharacter` null)
    (set `self.HasFallen` true)
    (bind _returnvalue (`self.K2_GetActorLocation` _asbp_third_person_character))
    (set `self.StepLocation` _returnvalue)
    (`KismetSystemLibrary.Delay` 0.2)
    (`PrimitiveComponent.SetSimulatePhysics` (`self.StaticMesh`) true)
    (`PrimitiveComponent.SetEnableGravity` (`self.StaticMesh`) true)
    (`KismetSystemLibrary.Delay` 0.2)
    (`self.K2_DetachFromActor` _asbp_third_person_character "KeepRelative" "KeepRelative" "KeepRelative")
    (`KismetSystemLibrary.Delay` 0.2)
    (`/Game/_01/BP/Player/BP_ThirdPersonCharacter.Die` _asbp_third_person_character)
    (`KismetSystemLibrary.Delay` 0.2)
    (`self.ResetFloor`)))

(event `self.Box4.OnComponentBeginOverlap`
  (params (OverlappedComponent :type "PrimitiveComponent Object Reference") (OtherActor :type "Actor Object Reference") (OtherComp :type "PrimitiveComponent Object Reference") (OtherBodyIndex :type Integer) (bFromSweep :type Boolean) (SweepResult :type "HitResult Structure (by ref)"))
  (if (not (`self.HasFallen`))
    (bind _asbp_third_person_character (cast `/Game/_01/BP/Player/BP_ThirdPersonCharacter` OtherActor))
    (set `self.AttachedCharacter` null)
    (set `self.HasFallen` true)
    (bind _returnvalue (`self.K2_GetActorLocation` _asbp_third_person_character))
    (set `self.StepLocation` _returnvalue)
    (`KismetSystemLibrary.Delay` 0.2)
    (`PrimitiveComponent.SetSimulatePhysics` (`self.StaticMesh`) true)
    (`PrimitiveComponent.SetEnableGravity` (`self.StaticMesh`) true)
    (`KismetSystemLibrary.Delay` 0.2)
    (`self.K2_DetachFromActor` _asbp_third_person_character "KeepRelative" "KeepRelative" "KeepRelative")
    (`KismetSystemLibrary.Delay` 0.2)
    (`/Game/_01/BP/Player/BP_ThirdPersonCharacter.Die` _asbp_third_person_character)
    (`KismetSystemLibrary.Delay` 0.2)
    (`self.ResetFloor`)))

(event `self.Box5.OnComponentBeginOverlap`
  (params (OverlappedComponent :type "PrimitiveComponent Object Reference") (OtherActor :type "Actor Object Reference") (OtherComp :type "PrimitiveComponent Object Reference") (OtherBodyIndex :type Integer) (bFromSweep :type Boolean) (SweepResult :type "HitResult Structure (by ref)"))
  (if (not (`self.HasFallen`))
    (bind _asbp_third_person_character (cast `/Game/_01/BP/Player/BP_ThirdPersonCharacter` OtherActor))
    (set `self.AttachedCharacter` null)
    (set `self.HasFallen` true)
    (bind _returnvalue (`self.K2_GetActorLocation` _asbp_third_person_character))
    (set `self.StepLocation` _returnvalue)
    (`KismetSystemLibrary.Delay` 0.2)
    (`PrimitiveComponent.SetSimulatePhysics` (`self.StaticMesh`) true)
    (`PrimitiveComponent.SetEnableGravity` (`self.StaticMesh`) true)
    (`KismetSystemLibrary.Delay` 0.2)
    (`self.K2_DetachFromActor` _asbp_third_person_character "KeepRelative" "KeepRelative" "KeepRelative")
    (`KismetSystemLibrary.Delay` 0.2)
    (`/Game/_01/BP/Player/BP_ThirdPersonCharacter.Die` _asbp_third_person_character)
    (`KismetSystemLibrary.Delay` 0.2)
    (`self.ResetFloor`)))

(event `self.Box6.OnComponentBeginOverlap`
  (params (OverlappedComponent :type "PrimitiveComponent Object Reference") (OtherActor :type "Actor Object Reference") (OtherComp :type "PrimitiveComponent Object Reference") (OtherBodyIndex :type Integer) (bFromSweep :type Boolean) (SweepResult :type "HitResult Structure (by ref)"))
  (if (not (`self.HasFallen`))
    (bind _asbp_third_person_character (cast `/Game/_01/BP/Player/BP_ThirdPersonCharacter` OtherActor))
    (set `self.AttachedCharacter` null)
    (set `self.HasFallen` true)
    (bind _returnvalue (`self.K2_GetActorLocation` _asbp_third_person_character))
    (set `self.StepLocation` _returnvalue)
    (`KismetSystemLibrary.Delay` 0.2)
    (`PrimitiveComponent.SetSimulatePhysics` (`self.StaticMesh`) true)
    (`PrimitiveComponent.SetEnableGravity` (`self.StaticMesh`) true)
    (`KismetSystemLibrary.Delay` 0.2)
    (`self.K2_DetachFromActor` _asbp_third_person_character "KeepRelative" "KeepRelative" "KeepRelative")
    (`KismetSystemLibrary.Delay` 0.2)
    (`/Game/_01/BP/Player/BP_ThirdPersonCharacter.Die` _asbp_third_person_character)
    (`KismetSystemLibrary.Delay` 0.2)
    (`self.ResetFloor`)))

(event `self.Box7.OnComponentBeginOverlap`
  (params (OverlappedComponent :type "PrimitiveComponent Object Reference") (OtherActor :type "Actor Object Reference") (OtherComp :type "PrimitiveComponent Object Reference") (OtherBodyIndex :type Integer) (bFromSweep :type Boolean) (SweepResult :type "HitResult Structure (by ref)"))
  (if (not (`self.HasFallen`))
    (bind _asbp_third_person_character (cast `/Game/_01/BP/Player/BP_ThirdPersonCharacter` OtherActor))
    (set `self.AttachedCharacter` null)
    (set `self.HasFallen` true)
    (bind _returnvalue (`self.K2_GetActorLocation` _asbp_third_person_character))
    (set `self.StepLocation` _returnvalue)
    (`KismetSystemLibrary.Delay` 0.2)
    (`PrimitiveComponent.SetSimulatePhysics` (`self.StaticMesh`) true)
    (`PrimitiveComponent.SetEnableGravity` (`self.StaticMesh`) true)
    (`KismetSystemLibrary.Delay` 0.2)
    (`self.K2_DetachFromActor` _asbp_third_person_character "KeepRelative" "KeepRelative" "KeepRelative")
    (`KismetSystemLibrary.Delay` 0.2)
    (`/Game/_01/BP/Player/BP_ThirdPersonCharacter.Die` _asbp_third_person_character)
    (`KismetSystemLibrary.Delay` 0.2)
    (`self.ResetFloor`)))

(event `self.Box1.OnComponentBeginOverlap`
  (params (OverlappedComponent :type "PrimitiveComponent Object Reference") (OtherActor :type "Actor Object Reference") (OtherComp :type "PrimitiveComponent Object Reference") (OtherBodyIndex :type Integer) (bFromSweep :type Boolean) (SweepResult :type "HitResult Structure (by ref)"))
  (if (not (`self.HasFallen`))
    (bind _asbp_third_person_character (cast `/Game/_01/BP/Player/BP_ThirdPersonCharacter` OtherActor))
    (set `self.AttachedCharacter` null)
    (set `self.HasFallen` true)
    (bind _returnvalue (`self.K2_GetActorLocation` _asbp_third_person_character))
    (set `self.StepLocation` _returnvalue)
    (`KismetSystemLibrary.Delay` 0.2)
    (`PrimitiveComponent.SetSimulatePhysics` (`self.StaticMesh`) true)
    (`PrimitiveComponent.SetEnableGravity` (`self.StaticMesh`) true)
    (`KismetSystemLibrary.Delay` 0.2)
    (`self.K2_DetachFromActor` _asbp_third_person_character "KeepRelative" "KeepRelative" "KeepRelative")
    (`KismetSystemLibrary.Delay` 0.2)
    (`/Game/_01/BP/Player/BP_ThirdPersonCharacter.Die` _asbp_third_person_character)
    (`KismetSystemLibrary.Delay` 30.2)
    (`self.ResetFloor`)))

(event `self.Box8.OnComponentBeginOverlap`
  (params (OverlappedComponent :type "PrimitiveComponent Object Reference") (OtherActor :type "Actor Object Reference") (OtherComp :type "PrimitiveComponent Object Reference") (OtherBodyIndex :type Integer) (bFromSweep :type Boolean) (SweepResult :type "HitResult Structure (by ref)"))
  (if (not (`self.HasFallen`))
    (bind _asbp_third_person_character (cast `/Game/_01/BP/Player/BP_ThirdPersonCharacter` OtherActor))
    (set `self.AttachedCharacter` null)
    (set `self.HasFallen` true)
    (bind _returnvalue (`self.K2_GetActorLocation` _asbp_third_person_character))
    (set `self.StepLocation` _returnvalue)
    (`KismetSystemLibrary.Delay` 0.2)
    (`PrimitiveComponent.SetSimulatePhysics` (`self.StaticMesh`) true)
    (`PrimitiveComponent.SetEnableGravity` (`self.StaticMesh`) true)
    (`KismetSystemLibrary.Delay` 0.2)
    (`self.K2_DetachFromActor` _asbp_third_person_character "KeepRelative" "KeepRelative" "KeepRelative")
    (`KismetSystemLibrary.Delay` 0.2)
    (`/Game/_01/BP/Player/BP_ThirdPersonCharacter.Die` _asbp_third_person_character)
    (`KismetSystemLibrary.Delay` 0.2)
    (`self.ResetFloor`)))

(event `self.Box16.OnComponentBeginOverlap`
  (params (OverlappedComponent :type "PrimitiveComponent Object Reference") (OtherActor :type "Actor Object Reference") (OtherComp :type "PrimitiveComponent Object Reference") (OtherBodyIndex :type Integer) (bFromSweep :type Boolean) (SweepResult :type "HitResult Structure (by ref)"))
  (if (not (`self.HasFallen`))
    (bind _asbp_third_person_character (cast `/Game/_01/BP/Player/BP_ThirdPersonCharacter` OtherActor))
    (set `self.AttachedCharacter` null)
    (set `self.HasFallen` true)
    (bind _returnvalue (`self.K2_GetActorLocation` _asbp_third_person_character))
    (set `self.StepLocation` _returnvalue)
    (`KismetSystemLibrary.Delay` 0.2)
    (`PrimitiveComponent.SetSimulatePhysics` (`self.StaticMesh`) true)
    (`PrimitiveComponent.SetEnableGravity` (`self.StaticMesh`) true)
    (`KismetSystemLibrary.Delay` 0.2)
    (`self.K2_DetachFromActor` _asbp_third_person_character "KeepRelative" "KeepRelative" "KeepRelative")
    (`KismetSystemLibrary.Delay` 0.2)
    (`/Game/_01/BP/Player/BP_ThirdPersonCharacter.Die` _asbp_third_person_character)
    (`KismetSystemLibrary.Delay` 0.2)
    (`self.ResetFloor`)))

(event `self.Box15.OnComponentBeginOverlap`
  (params (OverlappedComponent :type "PrimitiveComponent Object Reference") (OtherActor :type "Actor Object Reference") (OtherComp :type "PrimitiveComponent Object Reference") (OtherBodyIndex :type Integer) (bFromSweep :type Boolean) (SweepResult :type "HitResult Structure (by ref)"))
  (if (not (`self.HasFallen`))
    (bind _asbp_third_person_character (cast `/Game/_01/BP/Player/BP_ThirdPersonCharacter` OtherActor))
    (set `self.AttachedCharacter` null)
    (set `self.HasFallen` true)
    (bind _returnvalue (`self.K2_GetActorLocation` _asbp_third_person_character))
    (set `self.StepLocation` _returnvalue)
    (`KismetSystemLibrary.Delay` 0.2)
    (`PrimitiveComponent.SetSimulatePhysics` (`self.StaticMesh`) true)
    (`PrimitiveComponent.SetEnableGravity` (`self.StaticMesh`) true)
    (`KismetSystemLibrary.Delay` 0.2)
    (`self.K2_DetachFromActor` _asbp_third_person_character "KeepRelative" "KeepRelative" "KeepRelative")
    (`KismetSystemLibrary.Delay` 0.2)
    (`/Game/_01/BP/Player/BP_ThirdPersonCharacter.Die` _asbp_third_person_character)
    (`KismetSystemLibrary.Delay` 0.2)
    (`self.ResetFloor`)))

(event `self.Box14.OnComponentBeginOverlap`
  (params (OverlappedComponent :type "PrimitiveComponent Object Reference") (OtherActor :type "Actor Object Reference") (OtherComp :type "PrimitiveComponent Object Reference") (OtherBodyIndex :type Integer) (bFromSweep :type Boolean) (SweepResult :type "HitResult Structure (by ref)"))
  (if (not (`self.HasFallen`))
    (bind _asbp_third_person_character (cast `/Game/_01/BP/Player/BP_ThirdPersonCharacter` OtherActor))
    (set `self.AttachedCharacter` null)
    (set `self.HasFallen` true)
    (bind _returnvalue (`self.K2_GetActorLocation` _asbp_third_person_character))
    (set `self.StepLocation` _returnvalue)
    (`KismetSystemLibrary.Delay` 0.2)
    (`PrimitiveComponent.SetSimulatePhysics` (`self.StaticMesh`) true)
    (`PrimitiveComponent.SetEnableGravity` (`self.StaticMesh`) true)
    (`KismetSystemLibrary.Delay` 0.2)
    (`self.K2_DetachFromActor` _asbp_third_person_character "KeepRelative" "KeepRelative" "KeepRelative")
    (`KismetSystemLibrary.Delay` 0.2)
    (`/Game/_01/BP/Player/BP_ThirdPersonCharacter.Die` _asbp_third_person_character)
    (`KismetSystemLibrary.Delay` 0.2)
    (`self.ResetFloor`)))

(event `self.Box13.OnComponentBeginOverlap`
  (params (OverlappedComponent :type "PrimitiveComponent Object Reference") (OtherActor :type "Actor Object Reference") (OtherComp :type "PrimitiveComponent Object Reference") (OtherBodyIndex :type Integer) (bFromSweep :type Boolean) (SweepResult :type "HitResult Structure (by ref)"))
  (if (not (`self.HasFallen`))
    (bind _asbp_third_person_character (cast `/Game/_01/BP/Player/BP_ThirdPersonCharacter` OtherActor))
    (set `self.AttachedCharacter` null)
    (set `self.HasFallen` true)
    (bind _returnvalue (`self.K2_GetActorLocation` _asbp_third_person_character))
    (set `self.StepLocation` _returnvalue)
    (`KismetSystemLibrary.Delay` 0.2)
    (`PrimitiveComponent.SetSimulatePhysics` (`self.StaticMesh`) true)
    (`PrimitiveComponent.SetEnableGravity` (`self.StaticMesh`) true)
    (`KismetSystemLibrary.Delay` 0.2)
    (`self.K2_DetachFromActor` _asbp_third_person_character "KeepRelative" "KeepRelative" "KeepRelative")
    (`KismetSystemLibrary.Delay` 0.2)
    (`/Game/_01/BP/Player/BP_ThirdPersonCharacter.Die` _asbp_third_person_character)
    (`KismetSystemLibrary.Delay` 0.2)
    (`self.ResetFloor`)))

(event `self.Box12.OnComponentBeginOverlap`
  (params (OverlappedComponent :type "PrimitiveComponent Object Reference") (OtherActor :type "Actor Object Reference") (OtherComp :type "PrimitiveComponent Object Reference") (OtherBodyIndex :type Integer) (bFromSweep :type Boolean) (SweepResult :type "HitResult Structure (by ref)"))
  (if (not (`self.HasFallen`))
    (bind _asbp_third_person_character (cast `/Game/_01/BP/Player/BP_ThirdPersonCharacter` OtherActor))
    (set `self.AttachedCharacter` null)
    (set `self.HasFallen` true)
    (bind _returnvalue (`self.K2_GetActorLocation` _asbp_third_person_character))
    (set `self.StepLocation` _returnvalue)
    (`KismetSystemLibrary.Delay` 0.2)
    (`PrimitiveComponent.SetSimulatePhysics` (`self.StaticMesh`) true)
    (`PrimitiveComponent.SetEnableGravity` (`self.StaticMesh`) true)
    (`KismetSystemLibrary.Delay` 0.2)
    (`self.K2_DetachFromActor` _asbp_third_person_character "KeepRelative" "KeepRelative" "KeepRelative")
    (`KismetSystemLibrary.Delay` 0.2)
    (`/Game/_01/BP/Player/BP_ThirdPersonCharacter.Die` _asbp_third_person_character)
    (`KismetSystemLibrary.Delay` 0.2)
    (`self.ResetFloor`)))

(event `self.Box11.OnComponentBeginOverlap`
  (params (OverlappedComponent :type "PrimitiveComponent Object Reference") (OtherActor :type "Actor Object Reference") (OtherComp :type "PrimitiveComponent Object Reference") (OtherBodyIndex :type Integer) (bFromSweep :type Boolean) (SweepResult :type "HitResult Structure (by ref)"))
  (if (not (`self.HasFallen`))
    (bind _asbp_third_person_character (cast `/Game/_01/BP/Player/BP_ThirdPersonCharacter` OtherActor))
    (set `self.AttachedCharacter` null)
    (set `self.HasFallen` true)
    (bind _returnvalue (`self.K2_GetActorLocation` _asbp_third_person_character))
    (set `self.StepLocation` _returnvalue)
    (`KismetSystemLibrary.Delay` 0.2)
    (`PrimitiveComponent.SetSimulatePhysics` (`self.StaticMesh`) true)
    (`PrimitiveComponent.SetEnableGravity` (`self.StaticMesh`) true)
    (`KismetSystemLibrary.Delay` 0.2)
    (`self.K2_DetachFromActor` _asbp_third_person_character "KeepRelative" "KeepRelative" "KeepRelative")
    (`KismetSystemLibrary.Delay` 0.2)
    (`/Game/_01/BP/Player/BP_ThirdPersonCharacter.Die` _asbp_third_person_character)
    (`KismetSystemLibrary.Delay` 0.2)
    (`self.ResetFloor`)))

(event `self.Box10.OnComponentBeginOverlap`
  (params (OverlappedComponent :type "PrimitiveComponent Object Reference") (OtherActor :type "Actor Object Reference") (OtherComp :type "PrimitiveComponent Object Reference") (OtherBodyIndex :type Integer) (bFromSweep :type Boolean) (SweepResult :type "HitResult Structure (by ref)"))
  (if (not (`self.HasFallen`))
    (bind _asbp_third_person_character (cast `/Game/_01/BP/Player/BP_ThirdPersonCharacter` OtherActor))
    (set `self.AttachedCharacter` null)
    (set `self.HasFallen` true)
    (bind _returnvalue (`self.K2_GetActorLocation` _asbp_third_person_character))
    (set `self.StepLocation` _returnvalue)
    (`KismetSystemLibrary.Delay` 0.2)
    (`PrimitiveComponent.SetSimulatePhysics` (`self.StaticMesh`) true)
    (`PrimitiveComponent.SetEnableGravity` (`self.StaticMesh`) true)
    (`KismetSystemLibrary.Delay` 0.2)
    (`self.K2_DetachFromActor` _asbp_third_person_character "KeepRelative" "KeepRelative" "KeepRelative")
    (`KismetSystemLibrary.Delay` 0.2)
    (`/Game/_01/BP/Player/BP_ThirdPersonCharacter.Die` _asbp_third_person_character)
    (`KismetSystemLibrary.Delay` 0.2)
    (`self.ResetFloor`)))

(event `self.Box9.OnComponentBeginOverlap`
  (params (OverlappedComponent :type "PrimitiveComponent Object Reference") (OtherActor :type "Actor Object Reference") (OtherComp :type "PrimitiveComponent Object Reference") (OtherBodyIndex :type Integer) (bFromSweep :type Boolean) (SweepResult :type "HitResult Structure (by ref)"))
  (if (not (`self.HasFallen`))
    (bind _asbp_third_person_character (cast `/Game/_01/BP/Player/BP_ThirdPersonCharacter` OtherActor))
    (set `self.AttachedCharacter` null)
    (set `self.HasFallen` true)
    (bind _returnvalue (`self.K2_GetActorLocation` _asbp_third_person_character))
    (set `self.StepLocation` _returnvalue)
    (`KismetSystemLibrary.Delay` 0.2)
    (`PrimitiveComponent.SetSimulatePhysics` (`self.StaticMesh`) true)
    (`PrimitiveComponent.SetEnableGravity` (`self.StaticMesh`) true)
    (`KismetSystemLibrary.Delay` 0.2)
    (`self.K2_DetachFromActor` _asbp_third_person_character "KeepRelative" "KeepRelative" "KeepRelative")
    (`KismetSystemLibrary.Delay` 0.2)
    (`/Game/_01/BP/Player/BP_ThirdPersonCharacter.Die` _asbp_third_person_character)
    (`KismetSystemLibrary.Delay` 0.2)
    (`self.ResetFloor`)))

(fn `ResetFloor`
  (`PrimitiveComponent.SetSimulatePhysics` (`self.StaticMesh`) false)
  (`self.K2_SetActorLocation` (`self.InitialLocation`))
  (`self.K2_SetActorRotation` (`self.InitialRotation`))
  (set `self.HasFallen` false)
  (set `self.AttachedCharacter` null))

(fn `UserConstructionScript`)