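; Game mode for a parkour game that tracks checkpoints and handles level progression and restarts.
; On BeginPlay it gathers all BP_Checkpoint actors, takes the first as current, shows the main menu on "Main", and sets the character's ReverseControl only in Level_2.
; Checkpoint updates replace the current one; level completion increments the GameInstance index, then opens the next level by name after a delay, or Lvl_ThirdPerson past the last.
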(event `self.ReceiveBeginPlay`
  (`|ExecutionSequence`
    (:`then_0`
      (bind _outactors (`GameplayStatics.GetAllActorsOfClass` "/Game/_01/BP/Level/BP_Checkpoint.BP_Checkpoint_C"))
      (for _array_element _outactors
        (`KismetArrayLibrary.Array_Add` (`self.AllCheckpoints`) _array_element))
      (set `self.CurrentCheckpoint` (`|GetArrayItem` (`self.AllCheckpoints`))))
    (:`then_1`
      (bind _returnvalue (`GameplayStatics.GetCurrentLevelName` true))
      (if (`KismetStringLibrary.EqualEqual_StrStr` _returnvalue "Main")
        (bind _returnvalue_2 (`|CreateWidget` "/Game/_01/BP/UI/WBP_MainMenu.WBP_MainMenu_C"))
        (`UserWidget.AddToViewport` _returnvalue_2 0)))
    (:`then_2`
      (bind _returnvalue_3 (`GameplayStatics.GetCurrentLevelName` true))
      (if (`KismetStringLibrary.EqualEqual_StrStr` _returnvalue_3 "Level_2")
        (bind _asbp_third_person_character (cast `/Game/_01/BP/Player/BP_ThirdPersonCharacter` (`GameplayStatics.GetPlayerCharacter` 0)))
        (set `/Game/_01/BP/Player/BP_ThirdPersonCharacter.bReverseControl` true _asbp_third_person_character)
        (else
          (bind _asbp_third_person_character_2 (cast `/Game/_01/BP/Player/BP_ThirdPersonCharacter` (`GameplayStatics.GetPlayerCharacter` 0)))
          (set `/Game/_01/BP/Player/BP_ThirdPersonCharacter.bReverseControl` false _asbp_third_person_character_2))))))

(event `UpdateLastCheckpoint`
  (params (NewCheckpoint :type "/Game/_01/BP/Level/BP_Checkpoint Object Reference"))
  (set `self.CurrentCheckpoint` NewCheckpoint))

(event `OnLevelComplete`
  (bind _asbp_game_instance (cast `/Game/_01/BP/Gamemode/BP_GameInstance` (`GameplayStatics.GetGameInstance`)))
  (bind _result (`/Engine/EditorBlueprintResources/StandardMacros.IncrementInt` (`/Game/_01/BP/Gamemode/BP_GameInstance.CurrentLevelIndex` _asbp_game_instance))
    (:`  `
      (bind _output_get (set `/Game/_01/BP/Gamemode/BP_GameInstance.CurrentLevelIndex` _result _asbp_game_instance))
      (if (> _output_get (`self.TotalLevels`))
        (`GameplayStatics.OpenLevelBySoftObjectPtr` "/Game/ThirdPerson/Lvl_ThirdPerson.Lvl_ThirdPerson")
        (else
          (`KismetSystemLibrary.Delay` 1.0)
          (bind _levelname (`self.GetLevelNameByIndex` (`/Game/_01/BP/Gamemode/BP_GameInstance.CurrentLevelIndex` _asbp_game_instance)))
          (`GameplayStatics.OpenLevel` _levelname))))))

(event `RestartLevel`
  (bind _returnvalue (`GameplayStatics.GetCurrentLevelName` true))
  (`GameplayStatics.OpenLevel` (`KismetStringLibrary.Conv_StringToName` _returnvalue)))

(fn `GetLevelNameByIndex`
  (params (Index :type Integer))
  (returns (LevelName :type Name))
  (switch `int` Index
    (:`1`
      (return "Level_1"))
    (:`2`
      (return "Level_2"))
    (:`3`
      (return "Level_3"))))

(fn `UserConstructionScript`)