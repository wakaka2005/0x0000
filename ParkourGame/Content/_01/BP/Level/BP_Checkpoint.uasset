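; BP_Checkpoint is a parkour level checkpoint that the player character activates by overlapping it.
; On first overlap by BP_ThirdPersonCharacter it sets IsActivated, stores itself as the character's CurrentCheckpoint and turns on its particle effect.
; It then reports itself to BP_ParkourGameMode through UpdateLastCheckpoint.
; ResetCheckpoint clears the flag and deactivates the particles so it can trigger again.
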(event `self.ReceiveActorBeginOverlap`
  (params (OtherActor :type "Actor Object Reference"))
  ; 激活存档点
  (bind _asbp_third_person_character (cast `/Game/_01/BP/Player/BP_ThirdPersonCharacter` OtherActor))
  (if (not (`self.bIsActivated`))
    (set `self.bIsActivated` true)
    (set `/Game/_01/BP/Player/BP_ThirdPersonCharacter.CurrentCheckpoint` self _asbp_third_person_character)
    (`ActorComponent.Activate` (`self.ParticleSystem`) false)
    (bind _asbp_parkour_game_mode (cast `/Game/_01/BP/Gamemode/BP_ParkourGameMode` (`GameplayStatics.GetGameMode`)))
    (`/Game/_01/BP/Gamemode/BP_ParkourGameMode.UpdateLastCheckpoint` _asbp_parkour_game_mode self)))

(event `ResetCheckpoint`
  ; 重置存档点
  (set `self.bIsActivated` false)
  (`ActorComponent.Deactivate` (`self.ParticleSystem`)))

(fn `UserConstructionScript`)