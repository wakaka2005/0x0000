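; BP_TrapRevealManager is a level manager that reveals hidden traps one row at a time as progress advances.
; At BeginPlay it gathers actors tagged with each row number up to MaxRow, hides them and stores them per row.
; OnBoxTriggerOverlap reads the trigger's first tag as its row and reveals the following row, only if beyond CurrentRow.
; ResetTraps hides the stored traps again and zeroes CurrentRow.
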(event `self.ReceiveBeginPlay`
  (for _index (range 1 (+ (`self.MaxRow`) 1))
    (bind _output_get (set `self.TagString` (`KismetStringLibrary.Conv_IntToString` _index)))
    (bind _outactors (`GameplayStatics.GetAllActorsWithTag` (`KismetStringLibrary.Conv_StringToName` _output_get)))
    (bind _output_get_2 (set `self.TempArray` _outactors))
    (for _array_element _output_get_2
      (`self.SetActorHiddenInGame` _array_element true))
    (`KismetArrayLibrary.Array_Add` (`self.TrapRows`) (make `/Game/_01/BP/Data/FTrapRow` _index (`self.TempArray`)))))

(event `OnBoxTriggerOverlap`
  (params (BoxTriggerActor :type "Actor Object Reference"))
  (`/Engine/EditorBlueprintResources/StandardMacros.IsValid` BoxTriggerActor
    (:`Is Valid`
      (bind _output_get (set `self.BoxRow` (`KismetStringLibrary.Conv_StringToInt` (`KismetStringLibrary.Conv_NameToString` (`|GetArrayItem` (`Actor.Tags` BoxTriggerActor))))))
      (bind _output_get_2 (set `self.NextRow` (+ _output_get 1)))
      (if (> _output_get_2 (`self.CurrentRow`))
        (for _array_element (`self.TrapRows`)
          (if (== (break `/Game/_01/BP/Data/FTrapRow` _array_element) (`self.NextRow`))
            (`self.SetActorHiddenInGame` (`.TrapsArray_6_66B587EF4056940F21B5048B24C20C0C` (break `/Game/_01/BP/Data/FTrapRow` _array_element)) false)
            (set `self.CurrentRow` (`self.NextRow`))))))))

(event `ResetTraps`
  (for _array_element (`self.TrapRows`)
    (for _array_element_2 (`.TrapsArray_6_66B587EF4056940F21B5048B24C20C0C` (break `/Game/_01/BP/Data/FTrapRow` _array_element))
      (`self.SetActorHiddenInGame` _array_element_2 true)
      (set `self.CurrentRow` 0))))

(fn `UserConstructionScript`)