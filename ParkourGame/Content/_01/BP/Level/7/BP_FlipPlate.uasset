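; BP_FlipPlate is a level plate that flips when a BP_ThirdPersonCharacter with its Down flag set enters its trigger box.
; A timeline drives the mesh's relative pitch to flip it, then after a short delay a second timeline plays in reverse to return it.
; HasFlipped blocks re-triggering once the flip finishes, and the return clears both it and the character's Down flag.
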(event `self.Box.OnComponentBeginOverlap`
  (params (OverlappedComponent :type "PrimitiveComponent Object Reference") (OtherActor :type "Actor Object Reference") (OtherComp :type "PrimitiveComponent Object Reference") (OtherBodyIndex :type Integer) (bFromSweep :type Boolean) (SweepResult :type "HitResult Structure (by ref)"))
  (bind _asbp_third_person_character (cast `/Game/_01/BP/Player/BP_ThirdPersonCharacter` OtherActor))
  (if (`/Game/_01/BP/Player/BP_ThirdPersonCharacter.bDown` _asbp_third_person_character)
    (if (not (`self.bHasFlipped`))
      (bind (_direction `_新建轨道_0`) (`Timeline|TL_FlipPlate` :!via `PlayFromStart`)
        (:`Update`
          (`SceneComponent.K2_SetRelativeRotation` (`self.StaticMesh`) (`KismetMathLibrary.MakeRotator` 0.0 `_新建轨道_0`) false false))
        (:`Finished`
          (set `self.bHasFlipped` true)
          (`KismetSystemLibrary.Delay` 1.0)
          (bind (_direction_2 `_新建轨道_0_2`) (`Timeline|时间轴` :!via `ReverseFromEnd`)
            (:`Update`
              (`SceneComponent.K2_SetRelativeRotation` (`self.StaticMesh`) (`KismetMathLibrary.MakeRotator` 0.0 `_新建轨道_0_2`) false false))
            (:`Finished`
              (set `self.bHasFlipped` false)
              (set `/Game/_01/BP/Player/BP_ThirdPersonCharacter.bDown` false _asbp_third_person_character))))))))

(fn `UserConstructionScript`)