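; BP_HintTrigger is a one-shot level trigger that shows a hint on screen when overlapped.
; On the first actor overlap it sets HintShown, creates a WBP_hint widget, passes it the HintText and adds it to the viewport.
; After a fixed delay it removes the widget; the overlap does not check which actor entered.
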(event `self.ReceiveActorBeginOverlap`
  (params (OtherActor :type "Actor Object Reference"))
  ; 触碰调取提示UI
  (if (not (`self.HintShown`))
    (set `self.HintShown` true)
    (bind _returnvalue (`|CreateWidget` "/Game/_01/BP/UI/WBP_hint.WBP_hint_C"))
    (bind _output_get (set `self.NewVar` _returnvalue))
    (`/Game/_01/BP/UI/WBP_hint.SetHintText` _output_get (`self.HintText`))
    (`UserWidget.AddToViewport` (`self.NewVar`) 0)
    (`KismetSystemLibrary.Delay` 3.0)
    (`Widget.RemoveFromParent` (`self.NewVar`))))

(fn `UserConstructionScript`)