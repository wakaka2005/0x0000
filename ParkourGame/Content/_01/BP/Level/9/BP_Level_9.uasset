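; Level 9 actor that forces the player character back to a set location on a looping five-second timer.
; Each cycle plays a timeline that ramps post-process intensity, exposure compensation and vignette on a PostProcessVolume while driving a white camera fade with audio.
; When the timeline finishes, it moves the player to NewLocation, resets those post-process values and fades the view back in from white.
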(event `self.ReceiveBeginPlay`
  (`KismetSystemLibrary.K2_SetTimerDelegate` (delegate `ForceReturn`) 5.0 true))

(event `ForceReturn`
  (bind ((`SceneFringeIntensity` _scenefringeintensity) (`BloomIntensity` _bloomintensity) (`AutoExposureBias` _autoexposurebias) (`VignetteIntensity` _vignetteintensity)) (break `PostProcessSettings` (`PostProcessVolume.Settings` (`self.PostProcessVolume`))))
  (bind (_direction `_新建轨道_0`) (`Timeline|时间轴` :!via `PlayFromStart`)
    (:`Update`
      (`|ExecutionSequence`
        (:`then_0`
          (set `self.新建轨道 0` `_新建轨道_0`)
          (set `PostProcessVolume.Settings` (make `PostProcessSettings` :`SceneFringeIntensity` (`KismetMathLibrary.Lerp` _scenefringeintensity 10.0 (`self.新建轨道 0`)) :`BloomIntensity` (`KismetMathLibrary.Lerp` _bloomintensity 3.0 (`self.新建轨道 0`)) :`AutoExposureBias` (`KismetMathLibrary.Lerp` _autoexposurebias 0.8 (`self.新建轨道 0`)) :`VignetteIntensity` (`KismetMathLibrary.Lerp` _vignetteintensity 1.0 (`self.新建轨道 0`))) (`self.PostProcessVolume`)))
        (:`then_1`
          (`PlayerCameraManager.StartCameraFade` (`GameplayStatics.GetPlayerCameraManager` 0) 0.0 (`self.新建轨道 0`) 0.0 (struct :`R` 1.0 :`G` 1.0 :`B` 1.0 :`A` 1.0) true false))))
    (:`Finished`
      (`|ExecutionSequence`
        (:`then_0`
          (`self.K2_SetActorLocation` (`GameplayStatics.GetPlayerCharacter` 0) (`self.New Location`) false false))
        (:`then_1`
          (`KismetSystemLibrary.Delay` 0.2))
        (:`then_2`
          (set `PostProcessVolume.Settings` (make `PostProcessSettings` :`BloomIntensity` 0.0 :`AutoExposureBias` 0.0 :`VignetteIntensity` 0.0) (`self.PostProcessVolume`)))
        (:`then_3`
          (`PlayerCameraManager.StartCameraFade` (`GameplayStatics.GetPlayerCameraManager` 0) 1.0 0.0 0.5 (struct :`R` 1.0 :`G` 1.0 :`B` 1.0 :`A` 1.0) true false))))))

(fn `UserConstructionScript`)