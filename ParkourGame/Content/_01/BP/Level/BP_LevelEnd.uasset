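; BP_LevelEnd is a level-end trigger actor that shows the pass screen when the player character overlaps it.
; On overlap with BP_ThirdPersonCharacter, it disables input, adds the WBP_Pass widget to the viewport, pauses the game and switches to UI-only input with a visible cursor.
; A call to OnLevelComplete on BP_ParkourGameMode is present but unconnected, so the game mode is not notified.
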(event `self.ReceiveActorBeginOverlap`
  (params (OtherActor :type "Actor Object Reference"))
  (bind _returnvalue (`GameplayStatics.GetPlayerController` 0))
  (bind _asbp_third_person_character (cast `/Game/_01/BP/Player/Player_Pose/BP_ThirdPersonCharacter` OtherActor))
  (`self.DisableInput` _asbp_third_person_character (`GameplayStatics.GetPlayerController` 0))
  (bind _returnvalue_2 (`|CreateWidget` "/Game/_01/BP/UI/WBP_Pass.WBP_Pass_C"))
  (`UserWidget.AddToViewport` _returnvalue_2 0)
  (`GameplayStatics.SetGamePaused` true)
  (`WidgetBlueprintLibrary.SetInputMode_UIOnlyEx` _returnvalue null)
  (set `PlayerController.bShowMouseCursor` true _returnvalue))

(fn `UserConstructionScript`)