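; BP_DeathTrap_move is a trap that slides along its arrow once triggered and kills the player on contact.
; BeginPlay caches the start location and computes a target from the Arrow's forward vector and MoveDistance.
; The first player overlap with BoxMove plays a timeline that lerps the actor there without sweep, guarded by HasMoved so it fires once.
; Overlapping Boxkill calls Die on BP_ThirdPersonCharacter.
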(event `self.ReceiveBeginPlay`
  (set `self.StartLocation` (`self.K2_GetActorLocation`))
  (set `self.MoveDirection` (`SceneComponent.GetForwardVector` (`self.Arrow`)))
  (set `self.TargetLocation` (+ (`self.StartLocation`) (* (`self.MoveDistance`) (`self.MoveDirection`)))))

(event `self.Box move.OnComponentBeginOverlap`
  (params (OverlappedComponent :type "PrimitiveComponent Object Reference") (OtherActor :type "Actor Object Reference") (OtherComp :type "PrimitiveComponent Object Reference") (OtherBodyIndex :type Integer) (bFromSweep :type Boolean) (SweepResult :type "HitResult Structure (by ref)"))
  (cast `/Game/_01/BP/Player/BP_ThirdPersonCharacter` OtherActor)
  (if (not (`self.bHasMoved`))
    (set `self.bHasMoved` true)
    (bind (_direction `_新建轨道_1`) (`Timeline|时间轴` :!via `PlayFromStart`)
      (:`Update`
        (`self.K2_SetActorLocation` (`KismetMathLibrary.VLerp` (`self.StartLocation`) (`self.TargetLocation`) `_新建轨道_1`))))))

(event `self.Boxkill.OnComponentBeginOverlap`
  (params (OverlappedComponent :type "PrimitiveComponent Object Reference") (OtherActor :type "Actor Object Reference") (OtherComp :type "PrimitiveComponent Object Reference") (OtherBodyIndex :type Integer) (bFromSweep :type Boolean) (SweepResult :type "HitResult Structure (by ref)"))
  (bind _asbp_third_person_character (cast `/Game/_01/BP/Player/BP_ThirdPersonCharacter` OtherActor))
  (`/Game/_01/BP/Player/BP_ThirdPersonCharacter.Die` _asbp_third_person_character))

(fn `UserConstructionScript`)