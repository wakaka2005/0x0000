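; BP_RotatingObstacle is a trap actor that spins continuously and can kill the player character on contact.
; Tick adds a frame-rate independent local rotation built from RotationSpeed, RotationAxis and delta time.
; On actor overlap, if KillOnTouch is set, it casts the other actor to BP_ThirdPersonCharacter and calls Die.
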(event `self.ReceiveTick`
  (params (DeltaSeconds :type "Float (single-precision)"))
  (bind (_returnvalue_x _returnvalue_y _returnvalue_z) (`KismetMathLibrary.BreakVector` (* (* DeltaSeconds (`self.RotationSpeed`)) (`self.RotationAxis`))))
  (`self.K2_AddActorLocalRotation` (`KismetMathLibrary.MakeRotator` _returnvalue_x _returnvalue_y _returnvalue_z)))

(event `self.ReceiveActorBeginOverlap`
  (params (OtherActor :type "Actor Object Reference"))
  (if (`self.bKillOnTouch`)
    (bind _asbp_third_person_character (cast `/Game/_01/BP/Player/Player_Pose/BP_ThirdPersonCharacter` OtherActor))
    (`/Game/_01/BP/Player/Player_Pose/BP_ThirdPersonCharacter.Die` _asbp_third_person_character)))

(fn `UserConstructionScript`
  (`parent.UserConstructionScript`))